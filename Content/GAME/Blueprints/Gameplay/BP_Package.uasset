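; BP_Package is a physics pickup that the hero collects into a backpack, with a randomized InnerColor material parameter.
; On overlap, a timeline shrinks and flies it to the hero's backpack, then it teleports at full size above BP_Backpack and joins that actor's scene-capture show-only list.
; Events move it to the hero's Show point for removal or display, or shrink it into a given actor before destroying it.
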(event OnComponentHit(Sphere)
  (params (HitComponent :type Primitive%20Component%20Object%20Reference) (OtherActor :type Actor%20Object%20Reference) (OtherComp :type Primitive%20Component%20Object%20Reference) (NormalImpulse :type Vector :default "0, 0, 0") (Hit :type Hit%20Result%20Structure%20%28by%20ref%29)))

(event OnComponentBeginOverlap(Sphere)
  (params (OverlappedComponent :type Primitive%20Component%20Object%20Reference) (OtherActor :type Actor%20Object%20Reference) (OtherComp :type Primitive%20Component%20Object%20Reference) (OtherBodyIndex :type Integer) (bFromSweep :type Boolean) (SweepResult :type Hit%20Result%20Structure%20%28by%20ref%29))
  (bind _asbp_hero (Utilities|Casting|CastToBP_Hero OtherActor))
  (if (and (not (Variables|/Game/GAME/Blueprints/Core/BP_Hero.BP_Hero_C|GetbTakeSomething _asbp_hero)) (not (Variables|Default|GetbInBack)))
    (Utilities|FlowControl|DoOnce false :!label _label
      (:Completed
        (Physics|SetSimulatePhysics (Variables|Default|GetSphere) false)
        (Collision|SetActorEnableCollision false)
        (Variables|Default|SetNewVar (+ (Transformation|GetActorLocation) "0.000000,0.000000,150.000000"))
        (bind _asbp_hero_2 (Utilities|Casting|CastToBP_Hero (Game|GetPlayerCharacter 0)))
        (Class|BPIBackpack|Take(Message) _asbp_hero_2 true self)
        (Variables|Default|SetIcosphere (Variables|/Game/GAME/Blueprints/Core/BP_Hero.BP_Hero_C|GetBackpackMesh _asbp_hero_2))
        (bind _alpha (Timeline|Timeline PlayFromStart)
          (:Update
            (Transformation|SetActorLocation (Math|Vector|Lerp(Vector) (Variables|Default|GetNewVar) (+ (Transformation|GetWorldLocation (Variables|Default|GetIcosphere)) "0.000000,0.000000,150.000000") _alpha) false false)
            (Transformation|SetActorScale3D (Math|Vector|Lerp(Vector) "1.000000,1.000000,1.000000" "0.300000,0.300000,0.300000" _alpha)))
          (:Finished
            (bind _returnvalue (Actor|GetActorOfClass "/Game/GAME/Blueprints/Gameplay/BP_Backpack.BP_Backpack_C"))
            (Rendering|SceneCapture|ShowOnlyActorComponents (Variables|/Game/GAME/Blueprints/Gameplay/BP_Backpack.BP_Backpack_C|GetSceneCaptureComponent2D _returnvalue) self true)
            (Transformation|SetActorLocation (+ (Transformation|GetWorldLocation (Variables|/Game/GAME/Blueprints/Gameplay/BP_Backpack.BP_Backpack_C|GetMesh _returnvalue)) "0.000000,0.000000,600.000000") false true)
            (Physics|SetSimulatePhysics (Variables|Default|GetSphere) true)
            (Collision|SetActorEnableCollision true)
            (Transformation|SetActorScale3D "1.000000,1.000000,1.000000")
            (Variables|Default|SetbInBack true)
            (bind _asbp_hero_3 (Utilities|Casting|CastToBP_Hero (Game|GetPlayerCharacter 0)))
            (Class|BPIBackpack|Take(Message) _asbp_hero_3 false)
            (goto _label Reset)))))))

(event Custom|RemoveFromBack
  (Physics|SetSimulatePhysics (Variables|Default|GetSphere) true)
  (Collision|SetActorEnableCollision true)
  (bind _asbp_hero (Utilities|Casting|CastToBP_Hero (Game|GetPlayerCharacter 0)))
  (Transformation|SetActorLocation (Transformation|GetWorldLocation (Variables|/Game/GAME/Blueprints/Core/BP_Hero.BP_Hero_C|GetShow _asbp_hero)) false true)
  (Utilities|FlowControl|Delay 1.0)
  (Variables|Default|SetbInBack false))

(event Custom|Show
  (params (Show :type Boolean))
  (if Show
    (Variables|Default|SetNewVar (Transformation|GetActorLocation))
    (Variables|Default|SetbIsShowing true)
    (Physics|SetSimulatePhysics (Variables|Default|GetSphere) false)
    (Collision|SetActorEnableCollision false)
    (bind _asbp_hero (Utilities|Casting|CastToBP_Hero (Game|GetPlayerCharacter 0)))
    (Transformation|SetActorLocation (Transformation|GetWorldLocation (Variables|/Game/GAME/Blueprints/Core/BP_Hero.BP_Hero_C|GetShow _asbp_hero)) false true)
    (else
      (Transformation|SetActorLocation (Variables|Default|GetNewVar) false true)
      (Physics|SetSimulatePhysics (Variables|Default|GetSphere) true)
      (Collision|SetActorEnableCollision true))))

(event Custom|MouthDestroy
  (params (InputPin :type Actor%20Object%20Reference))
  (bind _self self)
  (bind _alpha (Timeline|Timeline_0 PlayFromStart)
    (:Update
      (Transformation|SetActorLocation _self (Math|Vector|Lerp(Vector) (Transformation|GetActorLocation _self) (Transformation|GetActorLocation InputPin) _alpha) false false)
      (Transformation|SetActorScale3D _self (Math|Vector|Lerp(Vector) "1.000000,1.000000,1.000000" "0.100000,0.100000,0.100000" _alpha)))
    (:Finished
      (Actor|DestroyActor _self))))

(fn ConstructionScript
  (Rendering|Material|SetVectorParameterValueonMaterials (Variables|Default|GetSphere) "InnerColor" (Math|Random|RandomUnitVector)))