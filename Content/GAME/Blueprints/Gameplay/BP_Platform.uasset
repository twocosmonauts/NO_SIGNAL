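; BP_Platform is a platform Blueprint that drastically boosts BP_Hero's speed while the hero overlaps its Box.
; Begin and end overlap write a high or normal value to the hero's NewVar, then copy it into MaxSpeed and MinSpeed.
; A Timeline that would move a second box along a Spline is never triggered, although the construction script still sets its play rate from Speed.
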(event OnComponentBeginOverlap(Box)
  (params (OverlappedComponent :type Primitive%20Component%20Object%20Reference) (OtherActor :type Actor%20Object%20Reference) (OtherComp :type Primitive%20Component%20Object%20Reference) (OtherBodyIndex :type Integer) (bFromSweep :type Boolean) (SweepResult :type Hit%20Result%20Structure%20%28by%20ref%29))
  (bind _asbp_hero (Utilities|Casting|CastToBP_Hero OtherActor))
  (bind _output_get (Variables|/Game/GAME/Blueprints/Core/BP_Hero.BP_Hero_C|SetNewVar _asbp_hero 1e+04))
  (bind _output_get_2 (Variables|/Game/GAME/Blueprints/Core/BP_Hero.BP_Hero_C|SetMaxSpeed _asbp_hero _output_get))
  (Variables|/Game/GAME/Blueprints/Core/BP_Hero.BP_Hero_C|SetMinSpeed _asbp_hero _output_get_2))

(event OnComponentEndOverlap(Box)
  (params (OverlappedComponent :type Primitive%20Component%20Object%20Reference) (OtherActor :type Actor%20Object%20Reference) (OtherComp :type Primitive%20Component%20Object%20Reference) (OtherBodyIndex :type Integer))
  (bind _asbp_hero (Utilities|Casting|CastToBP_Hero OtherActor))
  (bind _output_get (Variables|/Game/GAME/Blueprints/Core/BP_Hero.BP_Hero_C|SetNewVar _asbp_hero 3e+02))
  (bind _output_get_2 (Variables|/Game/GAME/Blueprints/Core/BP_Hero.BP_Hero_C|SetMaxSpeed _asbp_hero _output_get))
  (Variables|/Game/GAME/Blueprints/Core/BP_Hero.BP_Hero_C|SetMinSpeed _asbp_hero _output_get_2))

(fn ConstructionScript
  (Components|Timeline|SetPlayRate (Variables|Default|GetTimeline) (/ 1.0 (Variables|Default|GetSpeed))))