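; BP_MouthButton is a pressable button that makes the level's BP_Mouth actor say a phrase when BP_Hero steps into its trigger sphere.
; On overlap it plays a click and a timeline lowers the button mesh, then calls SayPhrase when fully pressed.
; Leaving the trigger reverses the timeline, and a DoOnce gate re-arms only after the button has fully risen.
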(event OnComponentBeginOverlap(Sphere1)
  (params (OverlappedComponent :type Primitive%20Component%20Object%20Reference) (OtherActor :type Actor%20Object%20Reference) (OtherComp :type Primitive%20Component%20Object%20Reference) (OtherBodyIndex :type Integer) (bFromSweep :type Boolean) (SweepResult :type Hit%20Result%20Structure%20%28by%20ref%29))
  (Utilities|Casting|CastToBP_Hero OtherActor)
  (Utilities|FlowControl|DoOnce false :!label _label
    (:Completed
      (Audio|SpawnSoundAttached "/Game/GAME/SOUNDS/Click.Click" (Variables|Default|GetSphere) "None" "0, 0, 0" "0, 0, 0" "KeepRelativeOffset" false 1.0 1.0 0.0 0 0)
      (bind (_direction _newtrack_0) (Timeline|PushButton Play)
        (:Update
          (Transformation|SetRelativeLocation (Variables|Default|GetSphere) (Math|Vector|MakeVector 0.0 0.0 (Math|Float|Lerp 0.0 -1e+01 _newtrack_0)) false false))
        (:Finished
          (switch Utilities|FlowControl|Switch|SwitchonETimelineDirection _direction
            (:Forward
              (bind _returnvalue (Actor|GetActorOfClass "/Game/GAME/Blueprints/Gameplay/BP_Mouth.BP_Mouth_C"))
              (Default|SayPhrase _returnvalue))
            (:Backward
              (goto _label Reset))))))))

(event OnComponentEndOverlap(Sphere1)
  (params (OverlappedComponent :type Primitive%20Component%20Object%20Reference) (OtherActor :type Actor%20Object%20Reference) (OtherComp :type Primitive%20Component%20Object%20Reference) (OtherBodyIndex :type Integer))
  (Utilities|Casting|CastToBP_Hero OtherActor)
  (bind (_direction _newtrack_0) (Timeline|PushButton Reverse)
    (:Update
      (Transformation|SetRelativeLocation (Variables|Default|GetSphere) (Math|Vector|MakeVector 0.0 0.0 (Math|Float|Lerp 0.0 -1e+01 _newtrack_0)) false false))
    (:Finished
      (switch Utilities|FlowControl|Switch|SwitchonETimelineDirection _direction
        (:Forward
          (bind _returnvalue (Actor|GetActorOfClass "/Game/GAME/Blueprints/Gameplay/BP_Mouth.BP_Mouth_C"))
          (Default|SayPhrase _returnvalue))
        (:Backward
          (Utilities|FlowControl|DoOnce false) ; enters at Reset
        )))))

(fn ConstructionScript)